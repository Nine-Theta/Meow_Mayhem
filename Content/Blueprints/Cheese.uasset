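; Cheese is a food pile actor that tracks how much cheese it holds.
; StealCheese lowers Amount by one, sets IsEmpty and prints a message once it reaches zero or below, and otherwise prints the remaining amount.
; AddCheese raises Amount by one without clearing IsEmpty.
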(event `StealCheese`
  (bind _output_get (set `self.Amount` (- (`self.Amount`) 1.0)))
  (if (<= _output_get 0.0)
    (set `self.isEmpty` true)
    (`KismetSystemLibrary.PrintString` "Foodpile is empty!")
    (else
      (`KismetSystemLibrary.PrintString` (`KismetStringLibrary.Conv_DoubleToString` _output_get)))))

(event `AddCheese`
  (set `self.Amount` (+ (`self.Amount`) 1.0)))

(fn `UserConstructionScript`)