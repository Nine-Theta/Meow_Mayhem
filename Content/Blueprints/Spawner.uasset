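; Spawner actor that creates mouse AI enemies at its location: stealer, ranged or buff, alone or as staggered stealer-and-buff groups.
; SpawnTimer calls SpawnMouse, which, when allowed, waits a random delay, then picks the type at random.
; CheckMouses pauses or resumes a spawn timer by comparing "Mouse"-tagged actors against MaxMouses.
; BeginPlay is empty and both looping timer setups are disconnected, so the spawner does not start itself.
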(event Custom|SpawnMouse
  (bind _returnvalue (Math|Random|RandomIntegerinRange 0 5))
  (if (Variables|Default|GetisAllowedToSpawn)
    (Utilities|FlowControl|Delay (Math|Random|RandomFloatinRange 0.1 (Variables|Default|GetSpawnRate)))
    (Development|PrintString (Utilities|String|ToString(Integer) _returnvalue))
    (switch int _returnvalue
      (:Default
        (CallFunction|SpawnStealer&Guard))
      (:0
        (CallFunction|SpawnStealer))
      (:1
        (CallFunction|SpawnRanged :!label _label))
      (:2
        (CallFunction|SpawnBuff))
      (:3
        (goto _label))
      (:4
        (CallFunction|SpawnStealer&Guard))
      (:5
        (CallFunction|SpawnStealer&DoubleGuard)))))

(event Custom|SpawnRanged
  (AI|SpawnAIFromClass "/Game/Graphic/Models/Characters/Rats/RangedMouse/RangedMouse_Character.RangedMouse_Character_C" 0 (Transformation|GetActorLocation) "0, 0, 0" false 0))

(event Custom|SpawnStealer&DoubleGuard
  (CallFunction|SpawnBuff)
  (Utilities|FlowControl|Delay 0.2)
  (CallFunction|SpawnStealer)
  (Utilities|FlowControl|Delay 0.8)
  (CallFunction|SpawnBuff))

(event Custom|SpawnStealer
  (AI|SpawnAIFromClass "/Game/Graphic/Models/Characters/Rats/StealerMouse/StealerMouse_Character.StealerMouse_Character_C" 0 (Transformation|GetActorLocation) "0, 0, 0" false 0))

(event Custom|SpawnBuff
  (AI|SpawnAIFromClass "/Game/Graphic/Models/Characters/Rats/BuffMouse/BuffMouse_Character.BuffMouse_Character_C" 0 (Transformation|GetActorLocation) "0, 0, 0" false 0))

(event Custom|DisableSpawner
  (Utilities|Time|PauseTimerbyHandle (stale _returnvalue)))

(event Custom|EnableSpawner
  (Utilities|Time|UnpauseTimerbyHandle (stale _returnvalue)))

(event Custom|CheckMouses
  (bind _outactors (Actor|GetAllActorswithTag "Mouse"))
  (if (> (Utilities|Array|Length _outactors) (Variables|Default|GetMaxMouses))
    (CallFunction|DisableSpawner)
    (else
      (CallFunction|EnableSpawner))))

(event Custom|SpawnStealer&Guard
  (CallFunction|SpawnStealer)
  (Utilities|FlowControl|Delay 0.2)
  (CallFunction|SpawnBuff))

(event EventBeginPlay)

(event Collision|EventActorBeginOverlap
  (params (OtherActor :type Actor%20Object%20Reference)))

(event EventTick
  (params (DeltaSeconds :type Float%20%28single-precision%29)))

(fn ConstructionScript)

(fn SpawnTimer
  (CallFunction|SpawnMouse))