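; Game instance that tracks score and game-over state and persists high-score data in the SaveData slot.
; Init loads or creates the save, a self-calling delayed timer and SCOREUP add points, and EndGame opens MenuPersistent.
; NeedsName picks the name-entry or end level by leaderboard place, and NameChange saves that name.
; The top-five ranking logic that sets the place is disconnected and never runs; NeedsNameChange is empty.
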(event `Init`
  (set `self.Score` 0)
  (bind _returnvalue (`GameplayStatics.DoesSaveGameExist` "SaveData"))
  (if _returnvalue
    (bind _returnvalue_2 (`GameplayStatics.LoadGameFromSlot` "SaveData"))
    (bind _assaved_data (cast `/Game/Blueprints/SavedData` _returnvalue_2))
    (set `self.HighScore` (`/Game/Blueprints/SavedData.HighScore` _assaved_data))
    (`GameplayStatics.SaveGameToSlot` _assaved_data "SaveData")
    (else
      (bind _returnvalue_3 (`GameplayStatics.CreateSaveGameObject` "/Game/Blueprints/SavedData.SavedData_C"))
      (set `/Game/Blueprints/SavedData.HighScore` (`self.HighScore`) _returnvalue_3)
      (`GameplayStatics.SaveGameToSlot` _returnvalue_3 "SaveData"))))

(event `ScoreTimer`
  (`KismetSystemLibrary.Delay` 1.0)
  (set `self.Score` (+ (`self.Score`) 5))
  (`self.ScoreTimer`))

(event `ResetScore`
  (set `self.Score` 0))

(event `SCOREUP`
  (params (`CustomAmount ?` :type Boolean) (CustomScoreAmount :type Integer))
  (bind _score (`self.Score`))
  (if `CustomAmount ?`
    (set `self.Score` (+ _score CustomScoreAmount))
    (else
      (set `self.Score` (+ _score (`self.ScoreUpAdd`))))))

(event `EndGame`
  (set `self.IsGameOver` true)
  (`GameplayStatics.OpenLevel` "MenuPersistent"))

(event `Needs Name`
  (switch `int` (`self.WhatPlace`)
    (:`Default`
      (`GameplayStatics.OpenLevel` "EndLevel" :!label _label))
    (:`0`
      (goto _label))
    (:`1`
      (`GameplayStatics.OpenLevel` "NameChangeLevel" :!label _label_2))
    (:`2`
      (goto _label_2))
    (:`3`
      (goto _label_2))
    (:`4`
      (goto _label_2))
    (:`5`
      (goto _label_2))))

(event `NameChange`
  (params (Name :type String))
  (bind _returnvalue (`GameplayStatics.LoadGameFromSlot` "SaveData"))
  (bind _assaved_data (cast `/Game/Blueprints/SavedData` _returnvalue))
  (switch `int` (`self.WhatPlace`)
    (:`1`
      (set `/Game/Blueprints/SavedData.Person1` Name _assaved_data))
    (:`2`
      (set `/Game/Blueprints/SavedData.Person2` Name _assaved_data))
    (:`3`
      (set `/Game/Blueprints/SavedData.Person3` Name _assaved_data))
    (:`4`
      (set `/Game/Blueprints/SavedData.Person4` Name _assaved_data))
    (:`5`
      (set `/Game/Blueprints/SavedData.Person5` Name _assaved_data)))
  (`GameplayStatics.SaveGameToSlot` _assaved_data (`/Game/Blueprints/SavedData.SaveSlotName` _assaved_data)))

(fn `NeedsNameChange`)