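; AI controller for the StealerMouse, a rat character that can carry cheese and senses the player.
; It runs BT_StealerMouse and, after a short delay, saves its own location to the blackboard as HoleLocation.
; Sight perception updates write the sensed-player flag and stimulus location to the blackboard; a distance-based tracking check is left unconnected.
; ReturnCheese, when cheese is held, adds it to the Cheese pile with the lowest amount.
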(event `self.ReceiveTick`
  (params (DeltaSeconds :type "Float (single-precision)")))

(event `Initialize`
  (params (Actor :type "/Game/Graphic/Models/Characters/Rats/StealerMouse/StealerMouse_Character Object Reference"))
  (set `self.Actor` Actor))

(event `self.ReceiveBeginPlay`
  ;[1 1 1] Initialize
  (`self.RunBehaviorTree` "/Game/Graphic/Models/Characters/Rats/StealerMouse/Blueprints/BT_StealerMouse.BT_StealerMouse")
  (`KismetSystemLibrary.Delay` 0.2)
  (`BlackboardComponent.SetValueAsVector` (`self.Blackboard`) (`self.HoleLocation`) (`self.K2_GetActorLocation`)))

(event `ReturnCheese`
  (bind _lowestcheesepile (`self.LowestCheesePile`))
  (if (`self.hasCheese`)
    (bind _outactors (`GameplayStatics.GetAllActorsOfClass` "/Game/Blueprints/Cheese.Cheese_C"))
    (for _array_element _outactors
      (`/Engine/EditorBlueprintResources/StandardMacros.IsValid` _lowestcheesepile
        (:`Is Valid`
          (if (< (`/Game/Blueprints/Cheese.Amount` _array_element) (`/Game/Blueprints/Cheese.Amount` _lowestcheesepile))
            (set `self.LowestCheesePile` _array_element)))
        (:`Is Not Valid`
          (set `self.LowestCheesePile` _array_element))))
    (`/Game/Blueprints/Cheese.AddCheese` (`self.LowestCheesePile`))))

(event `self.AIPerception.OnTargetPerceptionUpdated`
  (params (Actor :type "Actor Object Reference") (Stimulus :type "AIStimulus Structure"))
  (bind _outactors (`AIPerceptionComponent.GetCurrentlyPerceivedActors` (`self.AIPerception`) "/Script/AIModule.AISense_Sight"))
  ;[1 1 1] Update blackboard values
  (if (`KismetArrayLibrary.Array_IsValidIndex` _outactors)
    (for _array_element _outactors
      (bind _returnvalue (`self.ActorHasTag` _array_element "Player"))
      (if _returnvalue
        (break)))
    (if _returnvalue
      (`BlackboardComponent.SetValueAsVector` (`self.Blackboard`) (`self.SensedLocation`) (`.StimulusLocation` (break `AIStimulus` Stimulus)))
      (`BlackboardComponent.SetValueAsBool` (`self.Blackboard`) (`self.HasSensedSomething`) true)
      (else
        (`BlackboardComponent.SetValueAsBool` (`self.Blackboard`) (`self.HasSensedSomething`) false)))))

(fn `UserConstructionScript`)