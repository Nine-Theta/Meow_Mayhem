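; Anim notify for the ranged mouse that deals explosion damage around the animated character when it fires.
; It gathers every actor implementing the I_RatPickup interface and skips the mesh's owner.
; Any of those within a short fixed distance of the owner takes a small fixed amount of damage, using a manual distance check instead of radial damage or an overlap query.
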(fn `Received_Notify`
  (params (MeshComp :type "SkeletalMeshComponent Object Reference") (Animation :type "AnimSequenceBase Object Reference"))
  (returns (ReturnValue :type Boolean))
  (bind _returnvalue (`ActorComponent.GetOwner` MeshComp))
  (bind _outactors (`GameplayStatics.GetAllActorsWithInterface` "/Game/Scripts/Interfaces/I_RatPickup.I_RatPickup_C"))
  (for _array_element _outactors
    (if (!= _array_element _returnvalue)
      (if (< (`KismetMathLibrary.Vector_Distance` (`Actor.K2_GetActorLocation` _array_element) (`Actor.K2_GetActorLocation` _returnvalue)) 50.0)
        (`GameplayStatics.ApplyDamage` _array_element 1.0))))
  (return false))