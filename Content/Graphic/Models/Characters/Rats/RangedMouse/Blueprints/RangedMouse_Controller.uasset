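; AI controller for the RangedMouse enemy that runs BT_RangedMouse and feeds its blackboard.
; Sight perception records the sensed player, while a looping timer flags when a random player-tagged actor sits inside a distance band, neither too close nor too far.
; Attacks face the player and lock position before firing after a delay.
; An animation-notified forward line trace applies damage on a player hit, and the character's callback clears the attacking state.
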(event `LockRotation&Position`
  (if (not (`self.isAttacking`))
    (bind _outactors (`GameplayStatics.GetAllActorsWithTag` "Player"))
    (`self.SetLookatRotation` (`self.K2_GetActorLocation` (`KismetArrayLibrary.Array_Random` _outactors)))
    (`KismetSystemLibrary.Delay` 2.0)
    (set `self.isAttacking` true)
    (`BlackboardComponent.SetValueAsBool` (`self.Blackboard`) (`self.attacking`) true)
    (`/Game/Graphic/Models/Characters/Rats/RangedMouse/RangedMouse_Character.Attack` (`self.Actor`))))

(event `CheckDamageHit`
  (bind _actor (`self.Actor`))
  (bind _returnvalue (`self.K2_GetActorLocation` _actor))
  (bind _returnvalue_2 (`KismetMathLibrary.GetForwardVector` (`self.K2_GetActorRotation` _actor)))
  ;[1 1 1] Attack: Called from animation notification
  (bind _outhit (`KismetSystemLibrary.LineTraceSingle` (+ _returnvalue (* (`KismetMathLibrary.GetDirectionUnitVector` _returnvalue _returnvalue_2) 50.0)) (+ _returnvalue (* _returnvalue_2 5000.0)) "TraceTypeQuery1"))
  (if (`self.ActorHasTag` (`.HitActor` (`GameplayStatics.BreakHitResult` _outhit)) "Player")
    (`/Game/Graphic/Models/Characters/Rats/RangedMouse/RangedMouse_Character.DoDamage` (`self.Actor`))
    (else
      (`KismetSystemLibrary.PrintString` "Something?"))))

(event `SetLookatRotation`
  (params (TargetLookLocation :type "Vector Structure"))
  (bind _actor (`self.Actor`))
  (bind _returnvalue (`self.K2_GetActorLocation` _actor))
  ;[1 1 1] Set look rotation
  (`self.K2_SetActorRotation` _actor (`KismetMathLibrary.FindLookAtRotation` _returnvalue (`KismetMathLibrary.MakeVector` (.x TargetLookLocation) (.y TargetLookLocation) (.z _returnvalue))) false))

(event `self.ReceiveBeginPlay`
  ;[1 1 1] Start behaviour tree
  (`self.RunBehaviorTree` "/Game/Graphic/Models/Characters/Rats/RangedMouse/Blueprints/BT_RangedMouse.BT_RangedMouse"))

(event `AttackEnd`
  ;[1 1 1] Attack end: Called from character
  (set `self.isAttacking` false)
  (`BlackboardComponent.SetValueAsBool` (`self.Blackboard`) (`self.attacking`) false))

(event `Initialize`
  (params (Radius :type "Float (double-precision)") (Reference :type "/Game/Graphic/Models/Characters/Rats/RangedMouse/RangedMouse_Character Object Reference"))
  ;[1 1 1] Initialize blackboard values
  (`BlackboardComponent.SetValueAsFloat` (`self.Blackboard`) (`self.Radius`) Radius)
  (set `self.Actor` Reference)
  ;[1 1 1] Check if we are in attack range
  (`KismetSystemLibrary.K2_SetTimerDelegate` (delegate `CheckAttackRange`) 0.1 true))

(event `CheckAttackRange`
  (bind _returnvalue (`self.K2_GetActorLocation` (`self.Actor`)))
  ;[1 1 1] Check if we are in attack range
  (if (not (`self.isAttacking`))
    (bind _outactors (`GameplayStatics.GetAllActorsWithTag` "Player"))
    (if (`KismetArrayLibrary.Array_IsValidIndex` _outactors)
      (bind _returnvalue_2 (`self.K2_GetActorLocation` (`KismetArrayLibrary.Array_Random` _outactors)))
      (bind _returnvalue_3 (`KismetMathLibrary.Vector_Distance` _returnvalue_2 _returnvalue))
      (if (and (< _returnvalue_3 500.0) (> _returnvalue_3 250.0))
        (`BlackboardComponent.SetValueAsBool` (`self.Blackboard`) (`self.isInAttackRange`) true)
        (set `self.AttackDirection` (`KismetMathLibrary.GetDirectionUnitVector` _returnvalue _returnvalue_2))
        (else
          (`BlackboardComponent.SetValueAsBool` (`self.Blackboard`) (`self.isInAttackRange`) false))))))

(event `self.AIPerception.OnTargetPerceptionUpdated`
  (params (Actor :type "Actor Object Reference") (Stimulus :type "AIStimulus Structure"))
  (bind _outactors (`AIPerceptionComponent.GetCurrentlyPerceivedActors` (`self.AIPerception`) "/Script/AIModule.AISense_Sight"))
  ;[1 1 1] Set blackboard values based on perception
  (if (`self.isAttacking`)
    _
    (elif (`KismetArrayLibrary.Array_IsValidIndex` _outactors)
      ;;[1 1 1] Loop through all visible actors to check for player
      (for _array_element _outactors
        (bind _returnvalue (`self.ActorHasTag` _array_element "Player"))
        (if _returnvalue
          (break)))
      (if _returnvalue
        (`BlackboardComponent.SetValueAsObject` (`self.Blackboard`) (`self.Player`) _array_element)
        (`BlackboardComponent.SetValueAsBool` (`self.Blackboard`) (`self.HasSensedSomething`) true)
        (`BlackboardComponent.SetValueAsVector` (`self.Blackboard`) (`self.SensedLocation`) (`.StimulusLocation` (break `AIStimulus` Stimulus)))
        (else
          (`BlackboardComponent.SetValueAsBool` (`self.Blackboard`) (`self.HasSensedSomething`) false))))))

(fn `UserConstructionScript`)